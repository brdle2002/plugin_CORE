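; BP_UIManager is a UI manager Blueprint that, as written, only prints debug strings from its events.
; The game attributes update event calls its parent, then prints whether the updated tags include Action.Action, allowing non-exact matches.
; The initialized event prints a name with an initialization notice, and a separate GREETINGS event prints a hello message.
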(event EventOnGameAttributesUpdatedEvent
  (params (UpdatedTags :type Gameplay%20Tag%20Container%20Structure%20%28by%20ref%29))
  (|CallParentFunction UpdatedTags)
  (Development|PrintString 0 (Utilities|String|ToString(Boolean) (GameplayTags|HasTag UpdatedTags "(TagName=\"Action.Action\")"))))

(event EventOnInitializedEvent
  (Development|PrintString self (Utilities|String|Append (Variables|Default|GetName) " IS INITIALIZED")))

(event EventGREETINGS
  (Development|PrintString self))